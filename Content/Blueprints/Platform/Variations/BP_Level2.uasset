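; BP_Level2 is a platform variation that adds a BP_Prime_Helix actor to the level.
; On BeginPlay it always spawns the helix at the world transform of its PrimeHelixSpawnLocation component and stores the reference.
; When destroyed, it checks that reference, calls DestroyActor if it is valid, then runs the parent's Destroyed logic.
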(event EventBeginPlay
  (bind _returnvalue (Game|SpawnActorfromClass "/Game/Blueprints/Enemies/Prime_Helix/BP_Prime_Helix.BP_Prime_Helix_C" (Transformation|GetWorldTransform (Variables|Default|GetPrimeHelixSpawnLocation)) "AlwaysSpawn" 0 0)))

(event Collision|EventActorBeginOverlap
  (params (OtherActor :type Actor%20Object%20Reference))
  (|CallParentFunction OtherActor) ; This node is disabled and will not be called.\nDrag off pins to build functionality.
)

(event EventTick
  (params (DeltaSeconds :type Float%20%28single-precision%29))
  (|CallParentFunction DeltaSeconds) ; This node is disabled and will not be called.\nDrag off pins to build functionality.
)

(event EventDestroyed
  (Utilities|IsValid (stale EventBeginPlay _returnvalue)
    (:Is%20Valid
      (Actor|DestroyActor))
    (:Is%20Not%20Valid
      _))
  (|CallParentFunction))

(fn ConstructionScript
  (|CallParentFunction))