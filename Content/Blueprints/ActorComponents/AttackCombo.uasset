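; Actor component that sequences attack combos, each an array of attack function names with its own cycling counter.
; PerformCombo fires the current attack on the owner through a near-zero SetTimerByFunctionName, then advances the counter with wraparound.
; Calls made mid-attack set a single saved-attack flag, which PerformSavedAttack consumes to run the next attack.
; ResetCombo clears both state flags but leaves the counters untouched.
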(event Custom|PerformCombo
  (params (ComboIndex :type Integer))
  (bind _comboattacks (Variables|Default|GetComboAttacks))
  (bind _output (Utilities|Array|Get(acopy) _comboattacks ComboIndex))
  (bind _returnvalue (Utilities|Array|Length (.attacksinthiscombo _output)))
  (bind _output_2 (Utilities|Array|Get(acopy) (.attacksinthiscombo _output) (.currentattackcount _output)))
  (if (Variables|Default|GetIsAttacking)
    (Variables|Default|SetSaveAttack true)
    (CallFunction|SendDebugString "NewEnumerator2" "AttackComboComponent" "SavingAttack" 0.0 false false)
    (else
      (Variables|Default|SetIsAttacking true)
      (CallFunction|SendDebugString "NewEnumerator2" "AttackComboComponent" (Utilities|String|Append "Attack Performed: " _output_2) 0.0 false true)
      (Utilities|Time|SetTimerbyFunctionName (Components|GetOwner) _output_2 1e-06) ; TODO: Use interface?
      (|SetBy-RefVar (.currentattackcount _output) (Math|Integer|%(Integer) (+ (.currentattackcount _output) 1 _returnvalue) _returnvalue)))))

(event Custom|Reset%20Combo
  ;[1 1 1] Reset Combo
  (Variables|Default|SetIsAttacking false)
  (Variables|Default|SetSaveAttack false))

(event Custom|PerformSavedAttack
  (if (Variables|Default|GetSaveAttack)
    (Variables|Default|SetSaveAttack false)
    (Variables|Default|SetIsAttacking true)
    (CallFunction|SendDebugString "NewEnumerator2" "AttackComboComponent" (Utilities|String|Append "Attack Performed: " (Utilities|Array|Get(acopy) (.attacksinthiscombo (Utilities|Array|Get(acopy) (Variables|Default|GetComboAttacks) (stale Custom|PerformCombo ComboIndex))) (.currentattackcount (Utilities|Array|Get(acopy) (Variables|Default|GetComboAttacks) (stale Custom|PerformCombo ComboIndex))))) 0.0 false true)
    (Utilities|Time|SetTimerbyFunctionName (Components|GetOwner) (Utilities|Array|Get(acopy) (.attacksinthiscombo (Utilities|Array|Get(acopy) (Variables|Default|GetComboAttacks) (stale Custom|PerformCombo ComboIndex))) (.currentattackcount (Utilities|Array|Get(acopy) (Variables|Default|GetComboAttacks) (stale Custom|PerformCombo ComboIndex)))) 1e-06) ; TODO: Use interface?
    (|SetBy-RefVar (.currentattackcount (Utilities|Array|Get(acopy) (Variables|Default|GetComboAttacks) (stale Custom|PerformCombo ComboIndex))) (Math|Integer|%(Integer) (+ (.currentattackcount (Utilities|Array|Get(acopy) (Variables|Default|GetComboAttacks) (stale Custom|PerformCombo ComboIndex))) 1 (Utilities|Array|Length (.attacksinthiscombo (Utilities|Array|Get(acopy) (Variables|Default|GetComboAttacks) (stale Custom|PerformCombo ComboIndex))))) (Utilities|Array|Length (.attacksinthiscombo (Utilities|Array|Get(acopy) (Variables|Default|GetComboAttacks) (stale Custom|PerformCombo ComboIndex))))))))

(event EventBeginPlay)

(event EventTick
  (params (DeltaSeconds :type Float%20%28single-precision%29)))