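; Actor component that tracks whether superarmor is active on its owner, stored as a single boolean flag.
; Events turn the flag on or off, and a function exposes its current state to other Blueprints.
; A timed deactivation clears the flag and starts a one-shot timer that sets it back to true when the timeout ends, whatever the earlier state.
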(event Custom|ActivateSuperarmor
  (Variables|Default|SetSuperarmor true))

(event Custom|DeactivateSuperarmor
  (Variables|Default|SetSuperarmor false))

(event Custom|DeactivateSuperarmorWithTimeout
  (params (Timeout :type Float%20%28single-precision%29))
  (Variables|Default|SetSuperarmor false)
  (Utilities|Time|SetTimerbyEvent (delegate Custom|Reset) Timeout))

(event Custom|Reset
  (Variables|Default|SetSuperarmor true))

(event EventBeginPlay)

(event EventTick
  (params (DeltaSeconds :type Float%20%28single-precision%29)))

(fn IsSuperArmorActivated
  (return (Variables|Default|GetSuperarmor)))