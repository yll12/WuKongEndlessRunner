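; Actor component that makes its owner a hazard, hurting the player on touch.
; On BeginPlay it binds to the owner's begin-overlap event and prints each overlapping actor's name.
; For actors tagged Player, a DoOnce that is never reset applies fixed damage and sends a hit-react message with an impact particle system.
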(event Custom|CustomEvent_0
  (params (OverlappedActor :type Actor%20Object%20Reference) (OtherActor :type Actor%20Object%20Reference))
  (bind _returnvalue (Components|GetOwner))
  (Development|PrintString (Utilities|GetDisplayName OtherActor) false false)
  (if (Actor|ActorHasTag OtherActor "Player")
    (Utilities|FlowControl|DoOnce false
      (:Completed
        (Game|Damage|ApplyDamage OtherActor 22.0 0 _returnvalue)
        (Class|HitReactInterface|HitReact(Message) OtherActor _returnvalue (Variables|Default|GetImpact%20Particle%20System))))))

(event EventBeginPlay
  (Collision|BindEventtoOnActorBeginOverlap (Components|GetOwner) (delegate Custom|CustomEvent_0)))

(event EventTick
  (params (DeltaSeconds :type Float%20%28single-precision%29)))