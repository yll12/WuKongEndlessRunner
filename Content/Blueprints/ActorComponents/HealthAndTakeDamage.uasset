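; Actor component that gives its owner health and tracks damage taken.
; On BeginPlay it fills CurrentHealth from MaxHealth and binds to the owner's OnTakeAnyDamage event.
; Each hit subtracts damage, then prints a debug message if still alive or calls the CharacterHasDied dispatcher otherwise.
; IsAlive treats exactly zero health as alive, and nothing guards against repeated death calls.
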(event Custom|OnTakeAnyDamage_Event_0
  (params (DamagedActor :type Actor%20Object%20Reference) (Damage :type Float%20%28single-precision%29) (DamageType :type Damage%20Type%20Object%20Reference) (InstigatedBy :type Controller%20Object%20Reference) (DamageCauser :type Actor%20Object%20Reference))
  (Variables|Default|SetCurrentHealth (- (Variables|Default|GetCurrentHealth) Damage))
  (if (CallFunction|IsAlive)
    (Development|PrintString "Still ALive")
    (else
      (Default|CallCharacterHasDied))))

(event EventBeginPlay
  (Variables|Default|SetCurrentHealth (Variables|Default|GetMaxHealth))
  (EventDispatchers|AssignOnTakeAnyDamage (Components|GetOwner) (delegate Custom|OnTakeAnyDamage_Event_0)))

(fn IsAlive
  (return (>= (Variables|Default|GetCurrentHealth) 0.0)))