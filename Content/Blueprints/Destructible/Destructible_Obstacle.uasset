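; Destructible obstacle actor that swaps to an exploded version when damaged.
; The first damage received spawns Destructible_Obstacle_Exploded at the same transform, then hides the cube mesh and makes it ignore all collision.
; A separate one-shot HitReact event plays the supplied impact particles and sound, then destroys the actor after a short delay.
; An unconnected radius-damage branch with debug prints never runs.
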(event EventBeginPlay)

(event Collision|EventActorBeginOverlap
  (params (OtherActor :type Actor%20Object%20Reference)))

(event EventTick
  (params (DeltaSeconds :type Float%20%28single-precision%29)))

(event Game|Damage|EventAnyDamage
  (params (Damage :type Float%20%28single-precision%29) (DamageType :type Damage%20Type%20Object%20Reference) (InstigatedBy :type Controller%20Object%20Reference) (DamageCauser :type Actor%20Object%20Reference))
  (Utilities|FlowControl|DoOnce false
    (:Completed
      (Game|SpawnActorfromClass "/Game/Blueprints/Destructible/Destructible_Obstacle_Exploded.Destructible_Obstacle_Exploded_C" (Transformation|GetActorTransform) "AlwaysSpawn" 0 0)
      (Rendering|SetVisibility (Variables|Default|Get1M_Cube_Chamfer_DM) false false)
      (Collision|SetCollisionResponsetoAllChannels (Variables|Default|Get1M_Cube_Chamfer_DM) "ECR_Ignore"))))

(event EventHitReact
  (params (damageCauser :type Actor%20Object%20Reference) (impactParticleSystem :type Impact%20Particle%20System%20Struct%20Structure%20%28by%20ref%29))
  (Utilities|FlowControl|DoOnce false
    (:Completed
      (Effects|SpawnEmitterAttached (.objref impactParticleSystem) (Variables|Default|Get1M_Cube_Chamfer_DM) "None" (.impactdesiredlocationoffset impactParticleSystem) (.impactdesiredrotation impactParticleSystem) (.impactdesiredscale impactParticleSystem) "SnapToTarget")
      (Audio|PlaySoundatLocation (.impactsoundeffect impactParticleSystem) (Transformation|GetActorLocation) "0, 0, 0" 1.0 1.0 0.0 0 0 0)
      (Utilities|FlowControl|Delay 5.0)
      (Actor|DestroyActor))))

(fn ConstructionScript)