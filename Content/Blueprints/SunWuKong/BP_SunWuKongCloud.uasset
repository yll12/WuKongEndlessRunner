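; Sun WuKong's cloud actor, which renders a particle trail that can react to the movement of the actor it is attached to.
; BeginPlay spawns the scaled cloud emitter on its root.
; Each tick, when AdjustCloudPSToWuKongVelocity is on, the parent actor's speed drives spark and smoke spawn rates, and its velocity, with X forced negative, drives particle velocities.
; Otherwise it applies a default smoke-only stream.
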(event EventBeginPlay
  ;[1 1 1] Begin Play
  (bind _returnvalue (Effects|SpawnEmitterAttached "/Game/Assets/StarterContent/Particles/P_SunWuKongCloudParticles.P_SunWuKongCloudParticles" (Variables|Default|GetDefaultSceneRoot) "None" "-50.000000,0.000000,0.000000" "0, 0, 0" "8.000000,8.000000,8.000000"))
  (Variables|Default|SetCloud_ParticleSystem _returnvalue))

(event EventTick
  (params (DeltaSeconds :type Float%20%28single-precision%29))
  (bind _returnvalue (Actor|GetAttachParentActor))
  (bind _cloud_particlesystem (Variables|Default|GetCloud_ParticleSystem))
  ;[1 1 1] Event tick
  (if (Variables|Default|GetAdjustCloudPSToWuKongVelocity)
    (Utilities|IsValid _returnvalue
      (:Is%20Valid
        (CallFunction|SetParamAccordingtoVelocity _cloud_particlesystem _returnvalue)))
    (else
      (CallFunction|SetDefault _cloud_particlesystem))))

(fn ConstructionScript)

(fn SetDefault
  (params (CloudParticleSystem :type Particle%20System%20Component%20Object%20Reference))
  (Effects|Components|ParticleSystem|SetFloatParameter CloudParticleSystem "SparkSpawnRate" 0.0)
  (Effects|Components|ParticleSystem|SetFloatParameter CloudParticleSystem "SmokeSpawnRate" 5e+02)
  (Effects|Components|ParticleSystem|SetFloatParameter CloudParticleSystem "SparkBurstSpawnRate" 0.0)
  (Effects|Components|ParticleSystem|SetVectorParameter CloudParticleSystem "SparkInitialVelocity" "0, 0, 0")
  (Effects|Components|ParticleSystem|SetVectorParameter CloudParticleSystem "SmokeInitialVelocity" "-600.000000, 0, 0")
  (Effects|Components|ParticleSystem|SetVectorParameter CloudParticleSystem "SparkBurstSpawnRate" "0, 0, 0"))

(fn SetParamAccordingtoVelocity
  (params (Cloud%20Particle%20System :type Particle%20System%20Component%20Object%20Reference) (ParentActor :type Actor%20Object%20Reference))
  (bind _returnvalue (Transformation|GetVelocity ParentActor))
  (bind _returnvalue_2 (Math|Vector|VectorLength _returnvalue))
  (bind (_x _y _z) (Math|Vector|BreakVector _returnvalue))
  (bind _returnvalue_3 (Math|Float|Absolute(Float) _x))
  (bind _returnvalue_4 (* _returnvalue_3 -1.0))
  (bind _returnvalue_5 (Math|Vector|MakeVector _returnvalue_4 _y _z))
  (Effects|Components|ParticleSystem|SetFloatParameter Cloud%20Particle%20System "SparkSpawnRate" _returnvalue_2)
  (Effects|Components|ParticleSystem|SetFloatParameter Cloud%20Particle%20System "SmokeSpawnRate" _returnvalue_2)
  (Effects|Components|ParticleSystem|SetFloatParameter Cloud%20Particle%20System "SparkBurstSpawnRate" _returnvalue_2)
  (Effects|Components|ParticleSystem|SetVectorParameter Cloud%20Particle%20System "SparkInitialVelocity" _returnvalue_5)
  (Effects|Components|ParticleSystem|SetVectorParameter Cloud%20Particle%20System "SmokeInitialVelocity" _returnvalue_5)
  (Effects|Components|ParticleSystem|SetVectorParameter Cloud%20Particle%20System "SparkBurstSpawnRate" _returnvalue_5))