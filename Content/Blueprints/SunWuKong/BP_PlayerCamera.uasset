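; BP_PlayerCamera is a side-view follow camera that becomes player 0's view target on BeginPlay and tracks that player's pawn.
; Each Tick it holds Y at YOffset and sets X and Z through two dead-zone functions.
; Each axis stays put while the pawn is in range, otherwise snaps to the pawn's coordinate.
; The X range's upper bound is measured from world zero, unlike the camera-relative Z range.
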(event EventBeginPlay
  (Game|Player|SetViewTargetwithBlend (Game|GetPlayerController 0) self 0.0 "VTBlend_Linear" 0.0 false)
  (Variables|Default|SetActorToFollow (Game|Player|GetPlayerPawn 0)))

(event EventTick
  (params (DeltaSeconds :type Float%20%28single-precision%29))
  (Transformation|SetActorLocation (Math|Vector|MakeVector (CallFunction|GetNewXValue) (Variables|Default|GetYOffset) (CallFunction|GetNewZValue)) false false))

(fn ConstructionScript)

(fn GetNewXValue
  (bind _returnvalue (Transformation|GetActorLocation))
  (bind _actortofollow (Variables|Default|GetActorToFollow))
  (bind _xdeadzoneoffset (Variables|Default|GetXDeadZoneOffset))
  (bind _returnvalue_2 (Transformation|GetActorLocation _actortofollow))
  (if (Math|Float|InRange(Float) (.x _returnvalue_2) (- (.x _returnvalue) _xdeadzoneoffset) (+ 0.0 _xdeadzoneoffset))
    (return (.x _returnvalue))
    (else
      (return (.x _returnvalue_2)))))

(fn GetNewZValue
  (bind _returnvalue (Transformation|GetActorLocation))
  (bind _actortofollow (Variables|Default|GetActorToFollow))
  (bind _zdeadzoneoffset (Variables|Default|GetZDeadZoneOffset))
  (bind _returnvalue_2 (Transformation|GetActorLocation _actortofollow))
  (if (Math|Float|InRange(Float) (.z _returnvalue_2) (- (.z _returnvalue) _zdeadzoneoffset) (+ (.z _returnvalue) _zdeadzoneoffset))
    (return (.z _returnvalue))
    (else
      (return (.z _returnvalue_2)))))