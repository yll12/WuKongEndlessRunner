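; Component on the Sun Wukong character that toggles the summoned flying cloud, using a Toggle event fed the cloud collision and a timeline.
; Toggle spawns the cloud when activation is allowed, or, if one exists and deactivation is allowed, restores walking, jumps and resets the collision offset.
; The cloud's lerped fly-in and fly-out, switch to flying, destruction and flag re-enabling sit in disconnected nodes that never run.
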(event Custom|Toggle
  (params (Cloud%20Collision :type Box%20Component%20Object%20Reference) (Timeline :type Timeline%20Component%20Object%20Reference))
  ;[1 1 1] Toggle Flying
  (Variables|Default|SetCloud%20Collision Cloud%20Collision)
  (Variables|Default|SetTimeline Timeline)
  (Utilities|IsValid (Variables|Default|GetSunWuKongCloud)
    (:Is%20Valid
      (if (Variables|Default|GetCanDeactivateFly)
        (Variables|Default|SetCanDeactivateFly false)
        (Pawn|Components|CharacterMovement|SetMovementMode (Variables|Default|GetCharacter%20) "MOVE_Walking" 0)
        (Character|Jump (Variables|Default|GetAs%20Sun%20Wukong%20Character))
        (Transformation|SetRelativeLocation (Variables|Default|GetCloud%20Collision) "0, 0, 0" false true)
        (else
          (Development|PrintString "Cant Deactivate Cloud Yet!"))))
    (:Is%20Not%20Valid
      (if (Variables|Default|GetCanActivateFly)
        (Variables|Default|SetCanActivateFly false)
        (bind _returnvalue (Game|SpawnActorfromClass "/Game/Blueprints/SunWuKong/BP_SunWuKongCloud.BP_SunWuKongCloud_C" (Math|Transform|MakeTransform "0, 0, 0" "0, 0, 0" "1,1,1") "AdjustIfPossibleButAlwaysSpawn" 0 0))
        (bind _output_get (Variables|Default|SetSunWuKongCloud _returnvalue))
        (else
          (Development|PrintString "Fly on CD!!!!"))))))

(event EventBeginPlay
  (bind _assun_wukong_character (Utilities|Casting|CastToSunWukongCharacter (Components|GetOwner)))
  (Variables|Default|SetAs%20Sun%20Wukong%20Character _assun_wukong_character))