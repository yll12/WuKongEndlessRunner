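; Sun Wukong's cloud actor, which spawns an attached cloud particle system on BeginPlay.
; An event toggles whether Tick drives spawn rates from the parent actor's speed and initial velocities from its velocity, with X forced negative.
; With the toggle off, sparks stop and smoke uses a fixed rate and backward velocity.
; SparkBurstSpawnRate is written as both float and vector, with no burst velocity parameter set.
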(event Custom|AdjustCloudPSBasedOnVelocity
  (params (flag :type Boolean))
  (Variables|Default|SetAdjustCloudPSToWuKongVelocity flag))

(event EventBeginPlay
  (bind _returnvalue (Effects|SpawnEmitterAttached "/Game/Assets/StarterContent/Particles/P_SunWuKongCloudParticles.P_SunWuKongCloudParticles" (Variables|Default|GetDefaultSceneRoot) "None" "-50.000000,0.000000,0.000000" "0, 0, 0" "8.000000,8.000000,8.000000"))
  (Variables|Default|SetCloud_ParticleSystem _returnvalue))

(event EventTick
  (params (DeltaSeconds :type Float%20%28single-precision%29))
  (bind _returnvalue (Actor|GetAttachParentActor))
  (bind _cloud_particlesystem (Variables|Default|GetCloud_ParticleSystem))
  (bind _cloud_particlesystem_2 (Variables|Default|GetCloud_ParticleSystem))
  (bind _returnvalue_2 (Transformation|GetVelocity _returnvalue))
  (bind _returnvalue_3 (Math|Vector|VectorLength _returnvalue_2))
  (bind (_x _y _z) (Math|Vector|BreakVector _returnvalue_2))
  (bind _returnvalue_4 (Math|Float|Absolute(Float) _x))
  (bind _returnvalue_5 (* _returnvalue_4 -1.0))
  (bind _returnvalue_6 (Math|Vector|MakeVector _returnvalue_5 _y _z))
  (if (Variables|Default|GetAdjustCloudPSToWuKongVelocity)
    (Utilities|IsValid _returnvalue
      (:Is%20Valid
        (Effects|Components|ParticleSystem|SetFloatParameter _cloud_particlesystem "SparkSpawnRate" _returnvalue_3)
        (Effects|Components|ParticleSystem|SetFloatParameter _cloud_particlesystem "SmokeSpawnRate" _returnvalue_3)
        (Effects|Components|ParticleSystem|SetFloatParameter _cloud_particlesystem "SparkBurstSpawnRate" _returnvalue_3)
        (Effects|Components|ParticleSystem|SetVectorParameter _cloud_particlesystem "SparkInitialVelocity" _returnvalue_6)
        (Effects|Components|ParticleSystem|SetVectorParameter _cloud_particlesystem "SmokeInitialVelocity" _returnvalue_6)
        (Effects|Components|ParticleSystem|SetVectorParameter _cloud_particlesystem "SparkBurstSpawnRate" _returnvalue_6)))
    (else
      (Effects|Components|ParticleSystem|SetFloatParameter _cloud_particlesystem_2 "SparkSpawnRate" 0.0)
      (Effects|Components|ParticleSystem|SetFloatParameter _cloud_particlesystem_2 "SmokeSpawnRate" 5e+02)
      (Effects|Components|ParticleSystem|SetFloatParameter _cloud_particlesystem_2 "SparkBurstSpawnRate" 0.0)
      (Effects|Components|ParticleSystem|SetVectorParameter _cloud_particlesystem_2 "SparkInitialVelocity" "0, 0, 0")
      (Effects|Components|ParticleSystem|SetVectorParameter _cloud_particlesystem_2 "SmokeInitialVelocity" "-600.000000, 0, 0")
      (Effects|Components|ParticleSystem|SetVectorParameter _cloud_particlesystem_2 "SparkBurstSpawnRate" "0, 0, 0"))))

(fn ConstructionScript)